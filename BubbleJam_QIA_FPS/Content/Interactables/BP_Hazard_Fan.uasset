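; Fan hazard that continuously spins its blades and periodically pushes AI_Test enemies, apparently bubbled ones, caught in its influence capsule.
; A self-restarting timeline rotates the blade mesh, with play rate set by the interval length.
; After each revolution, overlapping enemies receive a push message carrying a force vector aimed from the actor's origin toward its Arrow component.
; The Construction Script sizes and offsets the capsule from configurable distance and girth.
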(event `self.ReceiveBeginPlay`
  (`self.BladeSpinningAnim`))

(event `BladeSpinningAnim`
  (`TimelineComponent.SetPlayRate` (`self.BladesSpin_Timeline`) (/ 1.0 (`self.IntervalLength`)))
  (bind (_direction _spin_alpha) (`Timeline|BladesSpin_Timeline` :!via `PlayFromStart`)
    (:`Update`
      (`SceneComponent.K2_SetRelativeRotation` (`self.FanBlades_Mesh`) (`KismetMathLibrary.MakeRotator` 0.0 (`KismetMathLibrary.Lerp` 0.0 360.0 _spin_alpha)) false false))
    (:`Finished`
      (`self.BladeSpinningAnim`)
      (`self.PushBubbledEnemy`))))

(event `PushBubbledEnemy`
  (bind _overlappingactors (`PrimitiveComponent.GetOverlappingActors` (`self.FanInfluence`) "/Game/AITesting/AI_Test.AI_Test_C"))
  (if (> (`KismetArrayLibrary.Array_Length` _overlappingactors) 0)
    (for _array_element _overlappingactors
      (message `/Game/BlueprintInterfaces/BPI_WeaponStrike.PushSignal` _array_element (* (`KismetMathLibrary.GetDirectionUnitVector` (`self.K2_GetActorLocation`) (`SceneComponent.K2_GetComponentLocation` (`self.Arrow`))) (`self.FanInfluenceForce`))))))

(fn `UserConstructionScript`
  (bind _faninfluence (`self.FanInfluence`))
  (`CapsuleComponent.SetCapsuleHalfHeight` _faninfluence (/ (`self.FanInfluenceDistance`) 2.0) true)
  (`CapsuleComponent.SetCapsuleRadius` _faninfluence (/ (`self.FanInfluenceGirth`) 2.0) true)
  (`SceneComponent.K2_SetRelativeLocation` _faninfluence (`KismetMathLibrary.MakeVector` 0.0 (/ (`self.FanInfluenceDistance`) 2.0) 283.0) false false))