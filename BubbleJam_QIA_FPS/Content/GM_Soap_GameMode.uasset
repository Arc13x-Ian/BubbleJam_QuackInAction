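; GM_Soap_GameMode is a game mode Blueprint that tracks the total kill count and a countdown timer for the HUD.
; UpdateKillCount increments TotalKills and passes it to HUDRef.
; StartTimer resets TimeRemaining to DefaultMaxTime and starts a looping 0.1-second timer that calls DecrementTimer.
; DecrementTimer subtracts each step and sends the time to the HUD as text, with no check for reaching zero.
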(event `/Game/BlueprintInterfaces/BPI_HUD_Update.UpdateKillCount`
  (params (KillCount :type Integer))
  (bind _result (`/Engine/EditorBlueprintResources/StandardMacros.IncrementInt` (`self.TotalKills`))
    (:`  `
      (`/Game/BlueprintInterfaces/BPI_HUD_Update.UpdateKillCount` (`self.HUDRef`) _result))))

(event `StartTimer`
  (set `self.TimeRemaining` (`self.DefaultMaxTime`))
  (`KismetSystemLibrary.K2_SetTimerDelegate` (delegate `DecrementTimer`) 0.1 true true))

(event `DecrementTimer`
  (bind _output_get (set `self.TimeRemaining` (- (`self.TimeRemaining`) 0.1)))
  (`/Game/BlueprintInterfaces/BPI_HUD_Update.UpdateTimeRemaining` (`self.HUDRef`) (`KismetStringLibrary.Conv_DoubleToString` _output_get)))

(fn `UserConstructionScript`)