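; BP_How_To_Play is a playground actor that displays how-to-play hints through text render components for movement, abilities and weapons.
; Its construction script tints the three weapon hints with WeaponTextColor and the sprint, dash, move, jump and suck hints with MovementTextColor.
; The event graph holds only disabled placeholder events, so the actor has no gameplay logic.
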(fn `UserConstructionScript`
  (`TextRenderComponent.SetTextRenderColor` (`self.How_To_Weapon3`) (`self.Weapon_Text_Color`))
  (`TextRenderComponent.SetTextRenderColor` (`self.How_To_Weapon2`) (`self.Weapon_Text_Color`))
  (`TextRenderComponent.SetTextRenderColor` (`self.How_To_Weapon1`) (`self.Weapon_Text_Color`))
  (`TextRenderComponent.SetTextRenderColor` (`self.How_To_Sprint`) (`self.Movement_Text_Color`))
  (`TextRenderComponent.SetTextRenderColor` (`self.How_To_Dash`) (`self.Movement_Text_Color`))
  (`TextRenderComponent.SetTextRenderColor` (`self.How_To_Move`) (`self.Movement_Text_Color`))
  (`TextRenderComponent.SetTextRenderColor` (`self.How_To_Jump`) (`self.Movement_Text_Color`))
  (`TextRenderComponent.SetTextRenderColor` (`self.How_To_Suck`) (`self.Movement_Text_Color`)))