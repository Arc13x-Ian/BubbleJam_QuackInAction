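; BP_Platform is a moving platform that shuttles back and forth between its starting relative location and EndLocation.
; After an initial delay, a timeline lerps the mesh component's relative location, with sweep off and a configurable play rate.
; Each time the timeline finishes, it waits a terminal delay, then checks its direction to play or reverse, looping endlessly.
; The construction script applies the configurable platform mesh.
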(event `self.ReceiveBeginPlay`
  (set `self.StartLocation` (`SceneComponent.RelativeLocation` (`self.Platform`)))
  (`TimelineComponent.SetPlayRate` (`self.TM_Platform_Move`) (`self.PlatformRate`))
  (`KismetSystemLibrary.Delay` (`self.InitialDelay`))
  (`self.Ev Go Forward`))

(event `Ev Go Forward`
  (bind (_direction _alpha) (`Timeline|TM_Platform_Move` :!label _label)
    (:`Update`
      (`SceneComponent.K2_SetRelativeLocation` (`self.Platform`) (`KismetMathLibrary.VLerp` (`self.StartLocation`) (`self.EndLocation`) _alpha) false false))
    (:`Finished`
      (`KismetSystemLibrary.Delay` (`self.TerminalDelay`))
      (if (`|EnumEquality` _direction "Forward")
        (`self.Ev Go Backward`)
        (else
          (`self.Ev Go Forward`))))))

(event `Ev Go Backward`
  (goto _label :!via `Reverse`))

(fn `UserConstructionScript`
  (`StaticMeshComponent.SetStaticMesh` (`self.Platform`) (`self.PlatformMesh`)))